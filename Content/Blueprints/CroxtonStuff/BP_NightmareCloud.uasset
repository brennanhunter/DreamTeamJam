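; BP_NightmareCloud is an AI enemy that chases pawns it sees and sends the player back to the start on contact.
; PawnSensing triggers AIMoveTo toward the seen pawn, with walk speed set from MaxSpeed at BeginPlay.
; Overlapping BP_ThirdPersonCharacter disables its movement, then after a short delay teleports it to the PlayerStart location with zero rotation.
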(event OnSeePawn(PawnSensing)
  (params (Pawn :type Pawn%20Object%20Reference))
  (AI|AIMoveTo self "0, 0, 0" Pawn 5.0 false))

(event EventBeginPlay
  (Variables|/Script/Engine.CharacterMovementComponent|SetMaxWalkSpeed (Variables|Character|GetCharacterMovement) (Variables|Default|GetMaxSpeed)))

(event Collision|EventActorBeginOverlap
  (params (OtherActor :type Actor%20Object%20Reference))
  (bind _asbp_third_person_character (Utilities|Casting|CastToBP_ThirdPersonCharacter OtherActor))
  (Variables|Default|SetCharacterRef _asbp_third_person_character)
  (if (== _asbp_third_person_character OtherActor)
    (Pawn|Components|CharacterMovement|DisableMovement (Variables|/Script/Engine.Character|GetCharacterMovement _asbp_third_person_character))
    (Utilities|FlowControl|Delay 0.3)
    (bind _returnvalue (Actor|GetActorOfClass "/Script/Engine.PlayerStart"))
    (Transformation|Teleport (Variables|Default|GetCharacterRef) (Transformation|GetActorLocation _returnvalue) "0, 0, 0")))

(fn ConstructionScript)