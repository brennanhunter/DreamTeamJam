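; BP_MovingPlatforms is a moving platform driven by an InterpToMovement component, with a configurable pause at one end of its travel.
; A FlipFlop on the component's reverse event alternates between restarting forward immediately and stopping for WaitBeforeReverse seconds.
; When that timer fires, the WaitTime event prints a debug "Hello" and restarts movement in the backward direction.
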(event OnInterptoReverse(InterpToMovement)
  (params (ImpactResult :type Hit%20Result%20Structure%20%28by%20ref%29) (Time :type Float%20%28single-precision%29))
  (Utilities|FlowControl|FlipFlop
    (:A
      (Components|Movement|StopMovementImmediately (Variables|Default|GetInterpToMovement))
      (Class|InterptoMovementComponent|RestartMovement (Variables|Default|GetInterpToMovement) 1.0))
    (:B
      (Components|Movement|StopMovementImmediately (Variables|Default|GetInterpToMovement))
      (Utilities|Time|SetTimerbyEvent (delegate Custom|WaitTime) (Variables|Default|GetWaitBeforeReverse)))))

(event Custom|WaitTime
  (Development|PrintString "Hello")
  (Class|InterptoMovementComponent|RestartMovement (Variables|Default|GetInterpToMovement) -1.0))

(fn ConstructionScript)